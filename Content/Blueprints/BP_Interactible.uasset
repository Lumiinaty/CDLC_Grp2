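; BP_Interactible is a grabbable world item that the player can interact with.
; Its Box overlap events show and hide the interact prompt on a BP_Player reference cached at BeginPlay.
; Grab returns the Cube's static mesh to the caller and triggers an event that destroys the actor after a short delay.
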(event OnComponentBeginOverlap(Box)
  (params (OverlappedComponent :type Primitive%20Component%20Object%20Reference) (OtherActor :type Actor%20Object%20Reference) (OtherComp :type Primitive%20Component%20Object%20Reference) (OtherBodyIndex :type Integer) (bFromSweep :type Boolean) (SweepResult :type Hit%20Result%20Structure%20%28by%20ref%29))
  ;[0.15 0.15 0.15 0.5] Interact text
  (bind _asbp_player (Utilities|Casting|CastToBP_Player OtherActor))
  (Utilities|IsValid _asbp_player
    (:Is%20Valid
      (Default|Show"Interact" (Variables|Default|GetPlayerREF)))))

(event OnComponentEndOverlap(Box)
  (params (OverlappedComponent :type Primitive%20Component%20Object%20Reference) (OtherActor :type Actor%20Object%20Reference) (OtherComp :type Primitive%20Component%20Object%20Reference) (OtherBodyIndex :type Integer))
  ;[0.15 0.15 0.15 0.5] Interact text
  (bind _asbp_player (Utilities|Casting|CastToBP_Player OtherActor))
  (Utilities|IsValid _asbp_player
    (:Is%20Valid
      (Default|Hide"Interact" (Variables|Default|GetPlayerREF)))))

(event Custom|Destroy%20Item%20To%20grab
  (Utilities|FlowControl|Delay 0.05)
  (Actor|DestroyActor))

(event EventBeginPlay
  ;[0.15 0.15 0.15 0.5] BeginPlay
  (bind _returnvalue (Actor|GetActorOfClass "/Game/TFPMovement/Player/Blueprints/BP_Player.BP_Player_C"))
  (Variables|Default|SetPlayerREF _returnvalue))

(fn ConstructionScript)

(fn Grab
  (CallFunction|DestroyItemtoGrab)
  (return (Variables|/Script/Engine.StaticMeshComponent|GetStaticMesh (Variables|Default|GetCube))))